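; BP_Geloctura is an AI character that chases the player and attacks with a punch.
; It stops its movement every tick until PawnSensing sees a pawn, then sets IsSeePlayer and runs FollowPlayer.
; FollowPlayer uses AIMoveTo toward the player character and, on success, plays the punch montage with a delayed CanAttack reset.
; IsSeePlayer is never cleared once set, and Patrol is an empty stub.
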(event OnSeePawn(PawnSensing)
  (params (Pawn :type Pawn%20Object%20Reference))
  (Variables|Default|SetIs%20See%20Player true)
  (CallFunction|FollowPlayer))

(event Custom|FollowPlayer
  (Variables|Default|SetCan%20Attack true)
  (if (Variables|Default|GetIs%20See%20Player)
    (AI|AIMoveTo self "0, 0, 0" (Game|GetPlayerCharacter 0) 7e+01 false
      (:OnSuccess
        (if (Variables|Default|GetCan%20Attack)
          (Variables|Default|SetCan%20Attack false)
          (Animation|PlayAnimMontage "/Game/_Eyderworld/Characteres/Gelocturas/Cross_Punch_Montage.Cross_Punch_Montage" 1.0 "None")
          (Utilities|FlowControl|Delay 2.0)
          (Variables|Default|SetCan%20Attack true))))
    (else
      (Variables|Default|SetIs%20See%20Player false))))

(event Custom|Patrol)

(event EventBeginPlay)

(event EventTick
  (params (DeltaSeconds :type Float%20%28single-precision%29))
  (if (not (Variables|Default|GetIs%20See%20Player))
    (Components|Movement|StopMovementImmediately (Variables|Character|GetCharacterMovement))))

(fn ConstructionScript)